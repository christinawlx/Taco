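; BP_FoodGenerator is a spawner actor that periodically drops a random food item into the level.
; On BeginPlay it fills the AllFood array with hamburger, hot dog, donut and taco classes, then starts a looping two-second timer bound to ThrowFood.
; ThrowFood spawns a random class from the array at the actor's root transform, always spawning regardless of collision.
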(event Custom|ThrowFood
  (Game|SpawnActorfromClass (Utilities|Array|Get(acopy) (Variables|Default|GetAllFood) (Math|Random|RandomIntegerinRange 0 3)) (Transformation|GetWorldTransform (Variables|Default|GetDefaultSceneRoot)) "AlwaysSpawn" 0 0))

(event EventBeginPlay
  (bind _allfood (Variables|Default|GetAllFood))
  (bind _allfood_2 (Variables|Default|GetAllFood))
  (Utilities|FlowControl|Sequence
    (:then_0
      (Utilities|Array|Add _allfood_2 "/Game/Bluprints/BP_Hamburger.BP_Hamburger_C"))
    (:then_1
      (Utilities|Array|Add _allfood_2 "/Game/Bluprints/BP_HotDog.BP_HotDog_C"))
    (:then_2
      (Utilities|Array|Add _allfood "/Game/Bluprints/BP_Donut.BP_Donut_C"))
    (:then_3
      (Utilities|Array|Add _allfood "/Game/Bluprints/BP_Taco.BP_Taco_C")
      (Utilities|Time|SetTimerbyEvent (delegate Custom|ThrowFood) 2.0 true))))

(event Collision|EventActorBeginOverlap
  (params (OtherActor :type Actor%20Object%20Reference)))

(event EventTick
  (params (DeltaSeconds :type Float%20%28single-precision%29)))

(fn ConstructionScript)
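; Base food actor that launches as a projectile along a randomized, mostly upward direction.
; The construction script calls Random, which gives the ProjectileMovement component a local-space velocity angled slightly toward negative Y by a random amount.
; The same function then sets both initial and max speed from the Speed variable.
; The event graph holds only disabled placeholder events, so all logic runs at construction.
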(event EventBeginPlay)

(event Collision|EventActorBeginOverlap
  (params (OtherActor :type Actor%20Object%20Reference)))

(event EventTick
  (params (DeltaSeconds :type Float%20%28single-precision%29)))

(fn ConstructionScript
  (CallFunction|Random))

(fn Random
  (bind _projectilemovement (Variables|Default|GetProjectileMovement))
  (bind _output_get (Variables|Default|Setdirection (Math|Vector|MakeVector 0.0 (Math|Random|RandomFloatinRange -0.4 -0.1) 1.0)))
  (Game|Components|ProjectileMovement|SetVelocityinLocalSpace (Variables|Default|GetProjectileMovement) _output_get)
  (Variables|/Script/Engine.ProjectileMovementComponent|SetInitialSpeed _projectilemovement (Variables|Default|Getspeed))
  (Variables|/Script/Engine.ProjectileMovementComponent|SetMaxSpeed _projectilemovement (Variables|Default|Getspeed)))
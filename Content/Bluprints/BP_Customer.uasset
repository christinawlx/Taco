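; BP_Customer is a customer actor that randomizes its appearance and a food index when play begins.
; RandomDecide hides the four variant components Apple, PokeGirl, Sim0801 and PokeBoy, then shows the one picked by a random TypeIndex.
; It also rolls FoodIndex independently from the same range, storing it without using it in this Blueprint.
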(event EventBeginPlay
  (CallFunction|RandomDecide))

(event Collision|EventActorBeginOverlap
  (params (OtherActor :type Actor%20Object%20Reference)))

(event EventTick
  (params (DeltaSeconds :type Float%20%28single-precision%29)))

(fn ConstructionScript)

(fn RandomDecide
  (bind _apple (Variables|Default|GetApple))
  (bind _poke_girl (Variables|Default|GetPoke_Girl))
  (bind _sim0801 (Variables|Default|Getsim0801))
  (bind _poke_boy (Variables|Default|GetPoke_Boy))
  (bind _array (Utilities|Array|MakeArray _apple _poke_girl _sim0801 _poke_boy))
  (for _array_element _array
    (Rendering|SetVisibility _array_element false false))
  (Variables|Default|SetFoodIndex (Math|Random|RandomIntegerinRange 0 3))
  (bind _output_get (Variables|Default|SetTypeIndex (Math|Random|RandomIntegerinRange 0 3)))
  (Rendering|SetVisibility (Utilities|Array|Get(acopy) _array _output_get) true false))
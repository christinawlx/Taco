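; Player character that slides sideways on horizontal input and catches food on a growing stack above its plate.
; When the Plate trigger overlaps food, it records the food type, destroys the item and attaches the matching mark actor at the stack top.
; Each catch stretches PlateTest by the food's box height and moves the trigger up to the Top component.
; CleanFood empties the stack and resets the plate.
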(event OnComponentBeginOverlap(Plate)
  (params (OverlappedComponent :type Primitive%20Component%20Object%20Reference) (OtherActor :type Actor%20Object%20Reference) (OtherComp :type Primitive%20Component%20Object%20Reference) (OtherBodyIndex :type Integer) (bFromSweep :type Boolean) (SweepResult :type Hit%20Result%20Structure%20%28by%20ref%29))
  (bind _platetest (Variables|Default|GetPlateTest))
  (bind _platetest_2 (Variables|Default|GetPlateTest))
  (bind _foodinhand (Variables|Default|GetFoodInHand))
  (bind _returnvalue (Transformation|GetWorldTransform _platetest_2))
  (bind _relativescale3d (Variables|/Script/Engine.SceneComponent|GetRelativeScale3D _platetest))
  (bind (_x _y _z) (Math|Vector|BreakVector _relativescale3d))
  (bind (_location _rotation) (Math|Transform|BreakTransform _returnvalue))
  (bind (_x_2 _y_2) (Math|Vector|BreakVector _location))
  (bind _asbp_food_parent (Utilities|Casting|CastToBP_FoodParent OtherActor))
  (Utilities|IsValid (Actor|GetComponentbyClass _asbp_food_parent "/Script/Engine.BoxComponent")
    (:Is%20Valid
      (bind _output_get (Variables|Default|SetTempHeight (.Z (Math|Vector|BreakVector (Variables|/Script/Engine.BoxComponent|GetBoxExtent (Actor|GetComponentbyClass _asbp_food_parent "/Script/Engine.BoxComponent"))))))
      (Utilities|Array|Add (Variables|Default|GetFoodInHand) (Variables|/Game/Bluprints/BP_FoodParent.BP_FoodParent_C|GetFoodType _asbp_food_parent))
      (Actor|DestroyActor OtherActor)
      (Transformation|SetRelativeScale3D (Variables|Default|GetPlateTest) (Math|Vector|MakeVector _x _y (+ _z _output_get)))
      (Transformation|SetWorldLocation (Variables|Default|GetPlate) (Transformation|GetWorldLocation (Variables|Default|GetTop)) false false)
      (bind _output_get_2 (Variables|Default|SetTopPointer (+ (Variables|Default|GetTopPointer) (* _output_get 2.0))))
      (bind _returnvalue_2 (Game|SpawnActorfromClass (Utilities|Array|Get(acopy) (Variables|Default|GetFoodMarks) (Utilities|Array|Get(acopy) _foodinhand (- (Utilities|Array|Length _foodinhand) 1))) (Math|Transform|MakeTransform (Math|Vector|MakeVector _x_2 _y_2 (- _output_get_2 _output_get)) _rotation) "AlwaysSpawn" 0 0))
      (Utilities|Array|Add (Variables|Default|GetMarkArray) _returnvalue_2)
      (Transformation|AttachActorToActor _returnvalue_2 self "None" "KeepWorld" "KeepWorld" "KeepWorld" true))))

(event EventBeginPlay
  (bind _foodmarks (Variables|Default|GetFoodMarks))
  (bind _foodmarks_2 (Variables|Default|GetFoodMarks))
  (Utilities|FlowControl|Sequence
    (:then_0
      (Utilities|Array|Add _foodmarks "/Game/Bluprints/BP_HamMark.BP_HamMark_C"))
    (:then_1
      (Utilities|Array|Add _foodmarks "/Game/Bluprints/BP_HotDogMark.BP_HotDogMark_C"))
    (:then_2
      (Utilities|Array|Add _foodmarks_2 "/Game/Bluprints/BP_DonutMark.BP_DonutMark_C"))
    (:then_3
      (Utilities|Array|Add _foodmarks_2 "/Game/Bluprints/BP_TacoMark.BP_TacoMark_C")
      (CallFunction|ResetTopPointer))))

(event EventTick
  (params (DeltaSeconds :type Float%20%28single-precision%29)))

(event Input|AxisEvents|InputAxisHorizontal
  (params (AxisValue :type Float%20%28single-precision%29))
  (Transformation|AddWorldOffset (Variables|Default|GetBox) (* "0,1.000000, 0" (* AxisValue (Variables|Default|GetSpeed))) true false))

(fn ConstructionScript)

(fn ResetTopPointer
  (Variables|Default|SetTopPointer (+ (.Z (Math|Vector|BreakVector (Transformation|GetWorldLocation (Variables|Default|GetPlateTest)))) 2.0))
  (Transformation|SetRelativeScale3D (Variables|Default|GetPlateTest) "1.000000,1.000000,1.000000")
  (Transformation|SetWorldLocation (Variables|Default|GetPlate) (Transformation|GetWorldLocation (Variables|Default|GetTop)) false false))

(fn CleanFood
  (Utilities|Array|Clear (Variables|Default|GetFoodInHand))
  (for _array_element (Variables|Default|GetMarkArray)
    (Actor|DestroyActor _array_element))
  (Utilities|Array|Clear (Variables|Default|GetMarkArray))
  (CallFunction|ResetTopPointer))
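; BP_ServingCube is a serving counter that queues customers and lets the player serve them food.
; A looping timer spawns BP_Customer actors at pivot transforms until the queue is full, passing each a reference to the counter.
; While BP_MainCharacter is inside the Box, a left click matches held food against each customer's FoodIndex.
; Matches remove food and customer, shift the queue along the pivots, and the player's food is re-sorted.
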(event OnComponentBeginOverlap(Box)
  (params (OverlappedComponent :type Primitive%20Component%20Object%20Reference) (OtherActor :type Actor%20Object%20Reference) (OtherComp :type Primitive%20Component%20Object%20Reference) (OtherBodyIndex :type Integer) (bFromSweep :type Boolean) (SweepResult :type Hit%20Result%20Structure%20%28by%20ref%29))
  (Utilities|Casting|CastToBP_MainCharacter OtherActor)
  (Variables|Default|SetCan_Serve true))

(event OnComponentEndOverlap(Box)
  (params (OverlappedComponent :type Primitive%20Component%20Object%20Reference) (OtherActor :type Actor%20Object%20Reference) (OtherComp :type Primitive%20Component%20Object%20Reference) (OtherBodyIndex :type Integer))
  (Utilities|Casting|CastToBP_MainCharacter OtherActor)
  (Variables|Default|SetCan_Serve false))

(event Custom|CreateCus
  (bind _curcus (Variables|Default|GetCurCus))
  (bind _custompivots (Variables|Default|GetCustomPivots))
  (bind _returnvalue (Utilities|Array|Length _curcus))
  (bind _output (Utilities|Array|Get(acopy) _custompivots _returnvalue))
  (bind _returnvalue_2 (Transformation|GetActorTransform _output))
  (bind (_location _rotation) (Math|Transform|BreakTransform _returnvalue_2))
  (if (< _returnvalue 5)
    (bind _returnvalue_3 (Game|SpawnActorfromClass "/Game/Bluprints/BP_Customer.BP_Customer_C" (Math|Transform|MakeTransform _location _rotation "4.500000,4.500000,4.500000") "Undefined" 0 0))
    (Utilities|Array|Add (Variables|Default|GetCurCus) _returnvalue_3)
    (Variables|/Game/Bluprints/BP_Customer.BP_Customer_C|SetservingRef _returnvalue_3 self)))

(event EventBeginPlay
  (Utilities|Time|SetTimerbyEvent (delegate Custom|CreateCus) 2.5 true))

(event Collision|EventActorBeginOverlap
  (params (OtherActor :type Actor%20Object%20Reference)))

(event EventTick
  (params (DeltaSeconds :type Float%20%28single-precision%29)))

(event Input|MouseEvents|LeftMouseButton
  (params (Key :type Key%20Structure))
  (:Pressed
    (if (Variables|Default|GetCan_Serve)
      (bind _asbp_main_character (Utilities|Casting|CastToBP_MainCharacter (Game|Player|GetPlayerPawn 0)))
      (bind _array_element (Utilities|Array|ForEachLoopwithBreak (Variables|Default|GetCurCus))
        (:LoopBody
          (bind (_array_element_2 _array_index) (Utilities|Array|ForEachLoopwithBreak (Variables|/Game/Bluprints/BP_MainCharacter.BP_MainCharacter_C|GetFoodInHand _asbp_main_character) :!label _label)
            (:LoopBody
              (if (== (Variables|/Game/Bluprints/BP_Customer.BP_Customer_C|GetFoodIndex _array_element) _array_element_2)
                (Default|RemoveFoodbyIndex _asbp_main_character _array_index)
                (CallFunction|RemoveCus _array_element)
                (CallFunction|ResetPosition)
                (goto _label Break)))))
        (:Completed
          (Default|SortFood _asbp_main_character))))))

(fn ConstructionScript)

(fn ResetPosition
  (for (_array_element _array_index) (Variables|Default|GetCurCus)
    (Transformation|SetActorLocation _array_element (Transformation|GetActorLocation (Utilities|Array|Get(acopy) (Variables|Default|GetCustomPivots) _array_index)) false false)))

(fn RemoveCus
  (params (Cus :type BP%20Customer%20Object%20Reference))
  (Utilities|Array|RemoveItem (Variables|Default|GetCurCus) Cus)
  (Actor|DestroyActor Cus))